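; Enemy spawner actor that spawns growing waves of BP_Zombie at its own transform.
; On BeginPlay it binds SpawnEnemy to the ThirdPersonGameMode's RespawnEnemy event.
; Each call waits through a delay, spawns the current count with collision adjustment, then raises the increment and adds it to the count, so waves grow at an accelerating rate.
; Nextwave_Event is only a debug print stub.
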(event Custom|SpawnEnemy
  (Utilities|FlowControl|Delay 5.0)
  (for _index (range 0 (- (Variables|Default|GetEnemySpawned) 1))
    (Game|SpawnActorfromClass "/Game/Enemies/BP_Zombie.BP_Zombie_C" (Transformation|GetActorTransform) "AdjustIfPossibleButAlwaysSpawn" 0 0))
  (Math|Integer|IncrementInt (Variables|Default|GetEnemyIncrement)
    (:%20%20
      (Variables|Default|SetEnemySpawned (+ (Variables|Default|GetEnemySpawned) (Variables|Default|GetEnemyIncrement))))))

(event Custom|Next%20wave_Event
  (Development|PrintString "Hello"))

(event EventBeginPlay
  (bind _asthird_person_game_mode (Utilities|Casting|CastToThirdPersonGameMode (Game|GetGameMode)))
  (EventDispatchers|BindEventtoRespawnEnemy _asthird_person_game_mode (delegate Custom|SpawnEnemy)))

(fn ConstructionScript)