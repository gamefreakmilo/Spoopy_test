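; BP_Zombie is an enemy that chases the player and destroys itself on contact, dealing damage.
; On BeginPlay it increments the game mode's EnemyAlive count and issues an AIMoveTo toward the player character.
; Hitting the player sends TakeDamageMessage, decrements EnemyAlive and calls CheckEnemyLeft before the zombie is destroyed.
; The pawn-sensing event is empty, and leftover zombie health and attack logic is disconnected.
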(event OnSeePawn(PawnSensing)
  (params (Pawn :type Pawn%20Object%20Reference)))

(event EventBeginPlay
  (bind _asthird_person_game_mode (Utilities|Casting|CastToThirdPersonGameMode (Game|GetGameMode)))
  (Math|Integer|IncrementInt (Variables|/Game/ThirdPersonBP/Blueprints/ThirdPersonGameMode.ThirdPersonGameMode_C|GetEnemyAlive _asthird_person_game_mode)
    (:%20%20
      (bind _asthird_person_character (Utilities|Casting|CastToThirdPersonCharacter (Game|GetPlayerCharacter 0)))
      (AI|AIMoveTo self "0, 0, 0" _asthird_person_character 5.0 false))))

(event Collision|EventHit
  (params (MyComp :type Primitive%20Component%20Object%20Reference) (Other :type Actor%20Object%20Reference) (OtherComp :type Primitive%20Component%20Object%20Reference) (bSelfMoved :type Boolean) (HitLocation :type Vector :default "0, 0, 0") (HitNormal :type Vector :default "0, 0, 0") (NormalImpulse :type Vector :default "0, 0, 0") (Hit :type Hit%20Result%20Structure%20%28by%20ref%29))
  (Utilities|Casting|CastToThirdPersonCharacter Other)
  (Class|BPIDamageable|TakeDamage(Message) Other 1e+01)
  (Utilities|Casting|CastToThirdPersonCharacter Other)
  (bind _asthird_person_game_mode (Utilities|Casting|CastToThirdPersonGameMode (Game|GetGameMode)))
  (Math|Integer|DecrementInt (Variables|/Game/ThirdPersonBP/Blueprints/ThirdPersonGameMode.ThirdPersonGameMode_C|GetEnemyAlive _asthird_person_game_mode)
    (:%20%20
      (Default|CheckEnemyLeft _asthird_person_game_mode)
      (Actor|DestroyActor))))

(event Input|ActionEvents|InputActionAttack
  (params (Key :type Key%20Structure :default "None")))

(event Input|MouseEvents|LeftMouseButton
  (params (Key :type Key%20Structure :default "None")))

(fn ConstructionScript)